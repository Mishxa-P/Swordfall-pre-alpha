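; Health component that tracks the current health of its owning actor and destroys that actor when health runs out.
; On BeginPlay it fills current health to the maximum.
; The ChangeHealth event subtracts the given amount, so negative values heal, and caps the result at maximum health.
; A result of zero or below destroys the owner directly, without updating the health value or notifying other systems.
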(event `self.ReceiveBeginPlay`
  (set `self.CurrentHealth` (`self.MaxHealth`)))

(event `ChangeHealth`
  (params (Amount :type Integer))
  (bind _maxhealth (`self.MaxHealth`))
  (bind _returnvalue (- (`self.CurrentHealth`) Amount))
  (if (<= (- (`self.CurrentHealth`) Amount) 0)
    (`Actor.K2_DestroyActor` (`self.GetOwner`))
    (elif (> _returnvalue _maxhealth)
      (set `self.CurrentHealth` _maxhealth)
      (else
        (set `self.CurrentHealth` _returnvalue)))))
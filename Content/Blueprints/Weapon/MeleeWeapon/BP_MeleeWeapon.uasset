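; BP_MeleeWeapon is a melee weapon with normal and great attacks.
; Both attacks sphere-overlap one object type just ahead of the owner, sized by AreaRadius, and change each hit actor's BP_Health_Component by Damage.
; NormalAttack also applies a mostly upward impulse to physics-simulating primitives, using only the forward vector's X horizontally.
; GreatAttack doubles Damage but applies no impulse.
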(fn `Apply Force`
  (params (Object :type "PrimitiveComponent Object Reference") (Location :type "Vector Structure"))
  (bind _returnvalue_x (`KismetMathLibrary.BreakVector` (`Actor.GetActorForwardVector` (`self.GetOwner`))))
  (if (`self.IsSimulatingPhysics` Object "None")
    (`self.AddImpulseAtLocation` Object (* (`KismetMathLibrary.MakeVector` _returnvalue_x 0.0 100.0) 1000) Location "None")))

(fn `GreatAttack`
  (bind _returnvalue (`self.GetOwner`))
  (bind _outactors (`KismetSystemLibrary.SphereOverlapActors` (+ (`Actor.K2_GetActorLocation` _returnvalue) (* (`Actor.GetActorForwardVector` _returnvalue) (`self.AreaRadius`))) (`self.AreaRadius`) (`|MakeArray` "ObjectTypeQuery8" :!type "EObjectTypeQuery Enum")))
  (for _array_element _outactors
    (`/Game/Blueprints/State/BP_Health_Component.ChangeHealth` (`Actor.GetComponentByClass` _array_element "/Game/Blueprints/State/BP_Health_Component.BP_Health_Component_C") (* (`self.Damage`) 2))))

(fn `NormalAttack`
  (bind _returnvalue (`self.GetOwner`))
  (bind _returnvalue_2 (+ (`Actor.K2_GetActorLocation` _returnvalue) (* (`Actor.GetActorForwardVector` _returnvalue) (`self.AreaRadius`))))
  (bind _outactors (`KismetSystemLibrary.SphereOverlapActors` _returnvalue_2 (`self.AreaRadius`) (`|MakeArray` "ObjectTypeQuery8" :!type "EObjectTypeQuery Enum")))
  (for _array_element _outactors
    (`self.Apply Force` (`Actor.GetComponentByClass` _array_element "/Script/Engine.PrimitiveComponent") _returnvalue_2)
    (`/Game/Blueprints/State/BP_Health_Component.ChangeHealth` (`Actor.GetComponentByClass` _array_element "/Game/Blueprints/State/BP_Health_Component.BP_Health_Component_C") (`self.Damage`))))